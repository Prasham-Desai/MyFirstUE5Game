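; BP_Target is a shootable Egyptian statue target.
; When a BP_ShooterProjectile_Bullet hits the statue mesh, an IsShot flag ensures it registers only once.
; The first hit swaps the material to M_Green and calls TargetShot on BP_ShooterGameMode to report it.
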(event `self.ReceiveBeginPlay`
  ; Lifecycle
  (`KismetSystemLibrary.PrintString` "Targer Spawned" true true (struct :`R` 1.0 :`B` 0.043637 :`A` 1.0)))

(event `self.Egyptian Statue.OnComponentHit`
  (params (HitComponent :type "PrimitiveComponent Object Reference") (OtherActor :type "Actor Object Reference") (OtherComp :type "PrimitiveComponent Object Reference") (NormalImpulse :type "Vector Structure") (Hit :type "HitResult Structure (by ref)"))
  ; Target Hitting Logic
  (cast `/Game/Variant_Shooter/Blueprints/Pickups/Projectiles/BP_ShooterProjectile_Bullet` OtherActor)
  (if (not (`self.IsShot`))
    (set `self.IsShot` true)
    (`PrimitiveComponent.SetMaterial` (`self.Egyptian Statue`) 0 "/Game/MyStuff/M_Green.M_Green")
    (bind _asbp_shooter_game_mode (cast `/Game/Variant_Shooter/Blueprints/BP_ShooterGameMode` (`GameplayStatics.GetGameMode`)))
    (`/Game/Variant_Shooter/Blueprints/BP_ShooterGameMode.TargetShot` _asbp_shooter_game_mode)))

(fn `UserConstructionScript`)